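; Civilian character Blueprint that can be infected and, while infected, makes itself audible to AI hearing.
; On BeginPlay it starts a looping one-second timer and calls Infect if the IsInfected flag is already set.
; The timer runs TestCall, which reports a noise event at the character's location whenever it is infected, with itself as instigator.
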(event `self.ReceiveBeginPlay`
  (`|ExecutionSequence`
    (:`then_0`
      (`KismetSystemLibrary.K2_SetTimer` null "TestCall" 1.0 true))
    (:`then_1`
      (if (`self.bIsInfected`)
        (`self.Infect`)))))

(fn `TestCall`
  (if (`self.bIsInfected`)
    (`AISense_Hearing.ReportNoiseEvent` (`self.K2_GetActorLocation`) 1.0 (`PawnMovementComponent.GetPawnOwner` (`self.CharacterMovement`)))))

(fn `UserConstructionScript`)