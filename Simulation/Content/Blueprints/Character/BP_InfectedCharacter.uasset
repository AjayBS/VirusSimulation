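; BP_InfectedCharacter is an AI-driven character that broadcasts its location as noise while infected.
; On BeginPlay it runs the InfectedBT behavior tree through its AI controller and starts a looping one-second timer on TestCall.
; TestCall checks IsInfected and, if set, reports an AI noise event at the actor's location with itself as instigator, feeding hearing perception.
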(event `self.ReceiveBeginPlay`
  (`KismetSystemLibrary.K2_SetTimer` null "TestCall" 1.0 true)
  (`AIController.RunBehaviorTree` (`AIBlueprintHelperLibrary.GetAIController` (`self.GetController`)) "/Game/Blueprints/AIEssentials/InfectedBT.InfectedBT"))

(fn `TestCall`
  (if (`self.bIsInfected`)
    (`AISense_Hearing.ReportNoiseEvent` (`self.K2_GetActorLocation`) 1.0 (`PawnMovementComponent.GetPawnOwner` (`self.CharacterMovement`)))))

(fn `UserConstructionScript`)