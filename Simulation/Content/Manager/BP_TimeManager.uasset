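; Time manager actor that runs an accelerated game clock and does some level setup on BeginPlay.
; BeginPlay switches the player's view to the level's CameraActor and stores all BP_NextTargetPoint actors in BP_GameManager's PlacesToHang.
; Tick accumulates scaled delta time into a Timespan, reading its hours component as Days and minutes as Hours, so a day spans 60 hours.
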(event `self.ReceiveBeginPlay`
  (`|ExecutionSequence`
    (:`then_0`
      (bind _returnvalue (`GameplayStatics.GetActorOfClass` "/Script/Engine.CameraActor"))
      (`PlayerController.SetViewTargetWithBlend` (`GameplayStatics.GetPlayerController` 0) _returnvalue 0.0 "VTBlend_Linear" 0.0 false))
    (:`then_1`
      (bind _outactors (`GameplayStatics.GetAllActorsOfClass` "/Game/Tasks/BP_NextTargetPoint.BP_NextTargetPoint_C"))
      (bind _asbp_game_manager (cast `/Game/Manager/BP_GameManager` (`GameplayStatics.GetGameInstance`)))
      (set `GameManager.PlacesToHang` _outactors _asbp_game_manager))))

(event `self.ReceiveTick`
  (params (DeltaSeconds :type "Float (single-precision)"))
  (bind _output_get (set `self.Tick` (+ (* DeltaSeconds 240.0) (`self.Tick`))))
  (bind _output_get_2 (set `self.Time` (`KismetMathLibrary.MakeTimespan` 0 0 0 (`KismetMathLibrary.FTrunc` _output_get))))
  (bind (_days _hours _minutes) (`KismetMathLibrary.BreakTimespan` _output_get_2))
  (set `self.Days` _hours)
  (set `self.Hours` _minutes))

(fn `UserConstructionScript`)