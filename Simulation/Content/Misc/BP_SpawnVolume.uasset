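; Spawn volume that populates the level with AI civilians on BeginPlay, in four counts combining infected and intellectual traits.
; SpawnCharacter offsets each randomly from the actor location within positive box extents, registers it with GameManager and rolls Kid, Youngster or OldAge through uneven nested random checks.
; Each loop then applies its traits, reports infected characters to GameManager and starts the civilian's behavior tree.
; The separate age-setting functions are empty stubs.
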(event `self.ReceiveBeginPlay`
  (`|ExecutionSequence`
    (:`then_0`
      (for _ (range 1 (+ (`self.InfectedAndNotIntellectual`) 1))
        (bind _character (`self.SpawnCharacter` true))
        (`CivilianCharacter.Infect` _character)
        (bind _asgame_manager (cast `GameManager` (`GameplayStatics.GetGameInstance`)))
        (`GameManager.SetCountOfInfectCharacters` _asgame_manager _character)
        (bind _ascivilian_controller (cast `CivilianController` (`Pawn.GetController` _character)))
        (`CivilianController.StartBehaviorTree` _ascivilian_controller)))
    (:`then_1`
      (for _ (range 1 (+ (`self.InfectedAndIntellectual`) 1))
        (bind _character_2 (`self.SpawnCharacter` true true))
        (`CivilianCharacter.Intellectual` _character_2)
        (`CivilianCharacter.Infect` _character_2)
        (cast `GameManager` (`GameplayStatics.GetGameInstance`))
        (`GameManager.SetCountOfInfectCharacters` _asgame_manager _character_2)
        (bind _ascivilian_controller_2 (cast `CivilianController` (`Pawn.GetController` _character_2)))
        (`CivilianController.StartBehaviorTree` _ascivilian_controller_2)))
    (:`then_2`
      (for _ (range 1 (+ (`self.NotInfectedAndNotIntellectual`) 1))
        (bind _character_3 (`self.SpawnCharacter` false))
        (bind _ascivilian_controller_3 (cast `CivilianController` (`Pawn.GetController` _character_3)))
        (`CivilianController.StartBehaviorTree` _ascivilian_controller_3)))
    (:`then_3`
      (for _ (range 1 (+ (`self.NotInfectedAndIntellectual`) 1))
        (bind _character_4 (`self.SpawnCharacter` false true))
        (`CivilianCharacter.Intellectual` _character_4)
        (bind _ascivilian_controller_4 (cast `CivilianController` (`Pawn.GetController` _character_4)))
        (`CivilianController.StartBehaviorTree` _ascivilian_controller_4)))
    (:`then_5`
      (`self.SettingAgeOfCharacters` null))))

(fn `SetAgeOfPeople`)

(fn `SettingAgeOfCharacters`
  (params (Character :type "/Game/Blueprints/Character/BP_CivilianCharacter Object Reference"))
  (locals (NoOfKids :type Integer) (NoOfYoungsters :type Integer) (NoOfAdults :type Integer)))

(fn `SpawnCharacter`
  (params (IsInfected :type Boolean) (IsIntellectual :type Boolean))
  (returns (Character :type "/Game/Blueprints/Character/BP_CivilianCharacter Object Reference"))
  (locals (CivilianCharacter :type "/Game/Blueprints/Character/BP_CivilianCharacter Object Reference"))
  (bind _returnvalue (`KismetMathLibrary.RandomIntegerInRange` 0 2))
  (bind _civiliancharacter (`local.CivilianCharacter`))
  (bind _returnvalue_2 (`AIBlueprintHelperLibrary.SpawnAIFromClass` "/Game/Blueprints/Character/BP_CivilianCharacter.BP_CivilianCharacter_C" null (+ (`KismetMathLibrary.MakeVector` (`KismetMathLibrary.RandomFloatInRange` 0.0 (.x (`BoxComponent.GetScaledBoxExtent` (`self.Volume`)))) (`KismetMathLibrary.RandomFloatInRange` 0.0 (.y (`BoxComponent.GetScaledBoxExtent` (`self.Volume`)))) (`KismetMathLibrary.RandomFloatInRange` 0.0 (.z (`BoxComponent.GetScaledBoxExtent` (`self.Volume`))))) (`self.K2_GetActorLocation`))))
  (bind _asbp_civilian_character (cast `/Game/Blueprints/Character/BP_CivilianCharacter` _returnvalue_2))
  (set `local.CivilianCharacter` _asbp_civilian_character)
  (bind _asgame_manager (cast `GameManager` (`GameplayStatics.GetGameInstance`)))
  (`GameManager.SetTotalCharacters` _asgame_manager _asbp_civilian_character)
  (if (== _returnvalue 0)
    (`GameManager.SetAgeOfCharacters` _asgame_manager _civiliancharacter "VE_Kid")
    (return _asbp_civilian_character)
    (elif (== _returnvalue 1)
      (`GameManager.SetAgeOfCharacters` _asgame_manager _civiliancharacter "VE_Youngster")
      (return _asbp_civilian_character)
      (elif true
        (`GameManager.SetAgeOfCharacters` _asgame_manager _civiliancharacter "VE_OldAge")
        (return _asbp_civilian_character)))))

(fn `UserConstructionScript`)